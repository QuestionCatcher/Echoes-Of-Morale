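; Player camera pawn providing free top-down style movement, zoom, rotation and screen-edge scrolling, with the cursor shown and locked to the viewport.
; Enhanced Input drives planar movement, clamped spring-arm zoom, and middle-mouse rotation that yaws the actor and pitches the arm.
; Mouse axis events push movement near viewport edges.
; Each tick, a downward visibility trace keeps the pawn at a set offset above the surface below.
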(event Input|EnhancedActionEvents|EnhancedInputActionIA_MoveAction
  (params (ActionValue :type Vector%202D%20Structure) (ElapsedSeconds :type Float%20%28double-precision%29) (TriggeredSeconds :type Float%20%28double-precision%29) (InputAction :type Input%20Action%20Object%20Reference :default "/Game/EchoesOfMorale/CameraSystem/Input/Actions/IA_MoveAction.IA_MoveAction"))
  (bind (_x _y) (Math|Vector2D|BreakVector2D ActionValue))
  ;[0.151 0.008653 0.1441 0.5] WASD Camera Movement
  (CallFunction|MoveForward _x)
  (CallFunction|MoveRight _y))

(event Input|EnhancedActionEvents|EnhancedInputActionIA_ZoomAction
  (params (ActionValue :type Float%20%28double-precision%29) (ElapsedSeconds :type Float%20%28double-precision%29) (TriggeredSeconds :type Float%20%28double-precision%29) (InputAction :type Input%20Action%20Object%20Reference :default "/Game/EchoesOfMorale/CameraSystem/Input/Actions/IA_ZoomAction.IA_ZoomAction"))
  (bind _springarm (Variables|Default|GetSpringArm))
  ;[0.151 0.008653 0.1441 0.5] Mouse Wheel Camera Zoom In/Out
  (Variables|/Script/Engine.SpringArmComponent|SetTargetArmLength _springarm (Math|Float|Clamp(Float) (+ (* ActionValue 5e+01) (Variables|/Script/Engine.SpringArmComponent|GetTargetArmLength _springarm)) 1e+02 1.5e+03)))

(event Input|EnhancedActionEvents|EnhancedInputActionIA_RotationAction
  (params (ActionValue :type Vector%202D%20Structure) (ElapsedSeconds :type Float%20%28double-precision%29) (TriggeredSeconds :type Float%20%28double-precision%29) (InputAction :type Input%20Action%20Object%20Reference :default "/Game/EchoesOfMorale/CameraSystem/Input/Actions/IA_RotationAction.IA_RotationAction"))
  (bind (_x _y) (Math|Vector2D|BreakVector2D ActionValue))
  (bind _returnvalue (Transformation|GetActorRotation))
  (bind _springarm (Variables|Default|GetSpringArm))
  (bind _returnvalue_2 (Class|SpringArmComponent|GetTargetRotation _springarm))
  (bind (_roll _pitch _yaw) (Math|Rotator|BreakRotator _returnvalue))
  (bind (_roll_2 _pitch_2 _yaw_2) (Math|Rotator|BreakRotator _returnvalue_2))
  ;[0.151 0.008653 0.1441 0.5] Camera Rotation by holding MMB + Mouse Move
  (if (Variables|Default|GetRotationActive)
    (Transformation|SetWorldRotation (Variables|Default|GetSpringArm) (Math|Rotator|MakeRotator 0.0 (Math|Float|Clamp(Float) (+ _y _pitch_2) -8e+01 -1e+01) _yaw_2) false false)
    (Transformation|SetActorRotation (Math|Rotator|MakeRotator 0.0 _pitch (Math|Float|Clamp(Float) (+ _yaw _x) -3.6e+02 3.6e+02)))))

(event EventTick
  (params (DeltaSeconds :type Float%20%28single-precision%29))
  (bind _returnvalue (Transformation|GetActorLocation))
  (bind _returnvalue_2 (Transformation|GetActorLocation))
  (bind _returnvalue_3 (Transformation|GetActorLocation))
  ;[0.151 0.008653 0.1441 0.5] Camera Z level adaptation based on hit result
  (bind _outhit (Collision|LineTraceByChannel (Math|Vector|MakeVector (.x _returnvalue_2) (.y _returnvalue_2) (+ (.z _returnvalue_2) (Variables|Default|GetDesireOffset))) (Math|Vector|MakeVector (.x _returnvalue) (.y _returnvalue) (+ (.z _returnvalue) -1e+03)) "TraceTypeQuery1" false 0 "None"))
  (Transformation|SetActorLocation (Math|Vector|MakeVector (.x _returnvalue_3) (.y _returnvalue_3) (+ (.Z (Math|Vector|BreakVector (.ImpactPoint (Collision|BreakHitResult _outhit)))) (Variables|Default|GetDesireOffset))) true false))

(event EventBeginPlay
  (Utilities|FlowControl|Sequence
    (:then_0
      (Input|SetInputModeGameandUI (Game|GetPlayerController 0) 0 "LockAlways" true false)
      (Variables|/Script/Engine.PlayerController|SetbShowMouseCursor (Game|GetPlayerController 0) true))))

(event Input|MouseEvents|MouseY
  (params (AxisValue :type Float%20%28single-precision%29))
  (bind _returnvalue (Game|GetPlayerController 0))
  (bind _returnvalue_2 (Viewport|GetViewportSize))
  (bind (_locationx _locationy) (Game|Player|GetMousePosition _returnvalue))
  (bind _returnvalue_3 (/ _locationx (.x _returnvalue_2)))
  ;[0.151 0.008653 0.1441 0.5] Camera Edge Scrolling
  (if (> _returnvalue_3 0.98)
    (CallFunction|MoveRight 1.0)
    (elif (< _returnvalue_3 0.02)
      (CallFunction|MoveRight -1.0))))

(event Input|MouseEvents|MouseX
  (params (AxisValue :type Float%20%28single-precision%29))
  (bind _returnvalue (Game|GetPlayerController 0))
  (bind _returnvalue_2 (Viewport|GetViewportSize))
  (bind (_locationx _locationy) (Game|Player|GetMousePosition _returnvalue))
  (bind _returnvalue_3 (/ _locationy (.y _returnvalue_2)))
  ;[0.151 0.008653 0.1441 0.5] Camera Edge Scrolling
  (if (> _returnvalue_3 0.98)
    (CallFunction|MoveForward -1.0)
    (elif (< _returnvalue_3 0.02)
      (CallFunction|MoveForward 1.0))))

(event Input|MouseEvents|MiddleMouseButton
  (params (Key :type Key%20Structure :default "None"))
  ;[0.151 0.008653 0.1441 0.5] Camera Rotation by holding MMB + Mouse Move
  (:Pressed
    (Variables|Default|SetRotationActive true))
  (:Released
    (Variables|Default|SetRotationActive false)))

(fn ConstructionScript)

(fn MoveForward
  (params (ScaleValue :type Float%20%28single-precision%29))
  (Pawn|Input|AddMovementInput (Transformation|GetActorForwardVector) ScaleValue false))

(fn MoveRight
  (params (ScaleValue :type Float%20%28single-precision%29))
  (Pawn|Input|AddMovementInput (Transformation|GetActorRightVector) ScaleValue false))