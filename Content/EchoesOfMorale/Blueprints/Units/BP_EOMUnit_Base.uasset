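; Base unit Blueprint for Echoes of Morale that can be selected, deselected and ordered to move to a location.
; Select and deselect events toggle the visibility of a selection decal.
; The move command stops the AI controller's current movement, then issues an AI MoveTo to the given location with a placeholder debug print.
; GrabSelectedUnits and the construction script are empty stubs.
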(event EventSelectUnit
  (Rendering|SetVisibility (Variables|Default|GetSelectionDecal) true false))

(event EventDeselectUnit
  (Rendering|SetVisibility (Variables|Default|GetSelectionDecal) false false))

(event EventUnitMoveCommand
  (params (Location :type Vector :default "0, 0, 0"))
  (bind _self self)
  (bind _returnvalue (AI|GetAIController _self))
  (AI|Navigation|StopMovement _returnvalue)
  (AI|AIMoveTo _returnvalue Location 0 -1.0 "Default" "Default" true true
    (:then
      (Development|PrintString "Hello"))))

(fn ConstructionScript)

(fn GrabSelectedUnits
  (return 0))